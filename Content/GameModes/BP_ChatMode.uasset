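; Game mode for a multiplayer chat-based number baseball game that relays messages and decides wins and draws.
; Each client message is rebroadcast to every BP_Controller, then checked by GameRule.
; A message containing "3 Strike" announces the sender as winner, while all players running out of RemainingChance announces a draw.
; Both outcomes call GameInitialize, as does BeginPlay, to restore chances and generate a new BaseballNumber.
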(event `self.ReceiveBeginPlay`
  (`self.GameInitialize`))

(event `GotMessageFromClient`
  (params (Msg :type String) (Controller :type "/Game/Blueprints/BP_Controller Object Reference"))
  (bind _outactors (`GameplayStatics.GetAllActorsOfClass` "/Script/Engine.PlayerController"))
  (for _array_element _outactors
    (bind _asbp_controller (cast `/Game/Blueprints/BP_Controller` _array_element))
    (`/Game/Blueprints/BP_Controller.GotBroadcast` _asbp_controller Msg))
  (`self.GameRule` Msg Controller))

(event `GameRule`
  (params (Msg :type String) (Controller :type "/Game/Blueprints/BP_Controller Object Reference"))
  (if (`KismetStringLibrary.Contains` Msg "3 Strike")
    (bind _outactors (`GameplayStatics.GetAllActorsOfClass` "/Script/Engine.PlayerController"))
    (for _array_element _outactors
      (bind _asbp_controller (cast `/Game/Blueprints/BP_Controller` _array_element))
      (`/Game/Blueprints/BP_Controller.GotBroadcast` _asbp_controller (`KismetTextLibrary.Conv_TextToString` (`|FormatText` "{Player} Win!!" (`/Game/Blueprints/BP_Controller.UserId` Controller))))
      (`self.GameInitialize`))
    (else
      (set `self.bIsDraw` true)
      (bind _outactors_2 (`GameplayStatics.GetAllActorsOfClass` "/Script/Engine.PlayerController"))
      (for _array_element_2 _outactors_2
        (bind _asbp_controller_2 (cast `/Game/Blueprints/BP_Controller` _array_element_2))
        (set `self.bIsDraw` (and (<= (`/Game/Blueprints/BP_Controller.RemainingChance` _asbp_controller_2) 0) (`self.bIsDraw`))))
      (if (`self.bIsDraw`)
        (bind _outactors_3 (`GameplayStatics.GetAllActorsOfClass` "/Script/Engine.PlayerController"))
        (for _array_element_3 _outactors_3
          (bind _asbp_controller_3 (cast `/Game/Blueprints/BP_Controller` _array_element_3))
          (`/Game/Blueprints/BP_Controller.GotBroadcast` _asbp_controller_3 "Game Over! Draw Game!!")
          (`self.GameInitialize`))))))

(event `GameInitialize`
  (bind _outactors (`GameplayStatics.GetAllActorsOfClass` "/Script/Engine.PlayerController"))
  (for _array_element _outactors
    (bind _asbp_controller (cast `/Game/Blueprints/BP_Controller` _array_element))
    (set `/Game/Blueprints/BP_Controller.RemainingChance` 3 _asbp_controller)
    (bind _returnvalue (`GenerateBaseBallNumber.GenerateBaseBall`))
    (set `self.BaseballNumber` _returnvalue)))

(fn `UserConstructionScript`)